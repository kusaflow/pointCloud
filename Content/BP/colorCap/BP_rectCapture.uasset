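; BP_rectCapture is an actor with a Plane and a Capture component, apparently a rectangular capture setup that positions itself from the plane's size.
; Its construction script places Capture at half of a 200-unit extent multiplied by the Plane's relative X and Z scale, with Y at zero.
; The position is set in world space without adding the actor's location, and the event graph holds no active logic.
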(fn `UserConstructionScript`
  (bind (_relativescale3d_x _relativescale3d_y _relativescale3d_z) (`KismetMathLibrary.BreakVector` (`SceneComponent.RelativeScale3D` (`self.plane`))))
  (bind _relativescale3d_x_2 (`KismetMathLibrary.BreakVector` (`SceneComponent.RelativeScale3D` (`self.plane`))))
  (`SceneComponent.K2_SetWorldLocation` (`self.capture`) (`KismetMathLibrary.MakeVector` (* (/ 50.0 100.0) (* 200 _relativescale3d_x_2)) 0.0 (* (/ 50.0 100.0) (* 200 _relativescale3d_z))) false false))