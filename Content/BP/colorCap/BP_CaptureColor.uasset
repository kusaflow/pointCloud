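; BP_CaptureColor is an actor Blueprint that, despite its name, contains only debug line-trace logic and no color capture.
; Its construction script traces on the Visibility channel forward from the Scencomp component and briefly draws the ray.
; The trace result is unused.
; The event graph is inactive, holding empty events and a disconnected, shorter copy of the same trace.
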(event `self.ReceiveTick`
  (params (DeltaSeconds :type "Float (single-precision)")))

(fn `UserConstructionScript`
  (bind _scencomp (`self.scencomp`))
  (bind _returnvalue (`SceneComponent.K2_GetComponentLocation` _scencomp))
  (`KismetSystemLibrary.LineTraceSingle` :`Start` _returnvalue :`End` (+ _returnvalue (* (`SceneComponent.GetForwardVector` _scencomp) 300.0)) :`TraceChannel` "TraceTypeQuery1" :`DrawDebugType` "ForDuration" :`DrawTime` 1.0))